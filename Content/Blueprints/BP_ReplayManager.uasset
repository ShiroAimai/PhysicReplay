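; Replay manager that counts down a minutes and seconds timer, then switches the game into replay and ends it when playback finishes.
; BeginPlay adds the replay widget, and a one-second Delay on Tick drives the countdown.
; At zero it sets the DRIVEN state and triggers the widget's replay event, with no guard against repeating.
; OnReplayedAllEntities shows the game-over widget and mouse cursor, then pauses the game.
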(event EventBeginPlay
  (bind _returnvalue (UserInterface|CreateWidget "/Game/Blueprints/UI/WBP_Replay.WBP_Replay_C"))
  (bind _output_get (Variables|Default|SetReplay%20Widget _returnvalue))
  (UserInterface|Viewport|AddtoViewport _output_get 0))

(event EventTick
  (params (DeltaSeconds :type Float%20%28single-precision%29))
  ;[1 1 1] Timer until replay kicks in
  (Utilities|FlowControl|Delay 1.0)
  (if (== (Variables|Default|GetSeconds) 0)
    (if (== (Variables|Default|GetMinutes) 0)
      ;[1 1 1] Init replay
      (Class|ReplayManager|SetState "REPLAY_DRIVEN")
      (Default|EventReplay (Variables|Default|GetReplay%20Widget))
      (else
        (Variables|Default|SetMinutes (- (Variables|Default|GetMinutes) 1))
        (Variables|Default|SetSeconds 59)))
    (else
      (Variables|Default|SetSeconds (- (Variables|Default|GetSeconds) 1)))))

(event EventOnReplayedAllEntities
  (bind _returnvalue (UserInterface|CreateWidget "/Game/Blueprints/UI/WBP_GameOver.WBP_GameOver_C"))
  (UserInterface|Viewport|AddtoViewport _returnvalue 0)
  (Variables|/Script/Engine.PlayerController|SetbShowMouseCursor (Game|GetPlayerController 0) true)
  (Game|SetGamePaused true))

(fn ConstructionScript)